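; BP_Hover is a player-controlled, physics-driven hover vehicle steered by two boosters on a Cube body.
; Forward input drives both boosters equally and Right input drives them oppositely, with Boost doubling thrust while held.
; At zero input, the boosters counter local forward velocity, and Booster2 alone counters yaw spin, giving automatic braking.
; Turn input yaws the SpringArm independently of the boosters.
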(event `InputAction|Boost`
  (params (Key :type "Key Structure"))
  (:`Pressed`
    (set `self.BoostMultiplier` 2.0))
  (:`Released`
    (set `self.BoostMultiplier` 1.0)))

(event `InputAxis|Turn`
  (params (AxisValue :type "Float (single-precision)"))
  (`SceneComponent.K2_AddRelativeRotation` (`self.SpringArm`) (`KismetMathLibrary.MakeRotator` 0.0 0.0 AxisValue) false false))

(event `InputAxis|Foreward`
  (params (AxisValue :type "Float (single-precision)"))
  (if (== AxisValue 0.0)
    (bind _returnvalue (`PrimitiveComponent.GetPhysicsLinearVelocity` (`self.Cube`) "None"))
    (bind _returnvalue_x (`KismetMathLibrary.BreakVector` (`KismetMathLibrary.InverseTransformDirection` (`self.GetTransform`) _returnvalue)))
    (`/Game/BP_Booster.Use` (`self.Booster 1`) (* _returnvalue_x -1.0))
    (`/Game/BP_Booster.Use` (`self.Booster 2`) (* _returnvalue_x -1.0))
    (else
      (`/Game/BP_Booster.Use` (`self.Booster 1`) (* AxisValue (`self.BoostMultiplier`)))
      (`/Game/BP_Booster.Use` (`self.Booster 2`) (* AxisValue (`self.BoostMultiplier`))))))

(event `InputAxis|Right`
  (params (AxisValue :type "Float (single-precision)"))
  (bind (_returnvalue_x _returnvalue_y _returnvalue_z) (`KismetMathLibrary.BreakVector` (`PrimitiveComponent.GetPhysicsAngularVelocityInDegrees` (`self.Cube`) "None")))
  (bind _returnvalue (* AxisValue (`self.BoostMultiplier`)))
  (if (== AxisValue 0.0)
    (`/Game/BP_Booster.Use` (`self.Booster 2`) (* _returnvalue_z -1.0))
    (`/Game/BP_Booster.Use` (`self.Booster 1`) 0.0)
    (else
      (`/Game/BP_Booster.Use` (`self.Booster 2`) _returnvalue)
      (`/Game/BP_Booster.Use` (`self.Booster 1`) (* _returnvalue -1.0)))))

(fn `UserConstructionScript`)