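; BP_HoverComponent is a hover suspension component that pushes its owning BP_Hover away from surfaces beneath it.
; Each tick it line-traces along its downward axis up to HoverDist and measures how far the hit compresses that distance.
; A spring-damper force from that compression and its rate of change is applied to the owner's root primitive at the component's location along its up vector.
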(event `self.ReceiveBeginPlay`
  (bind _asbp_hover (cast `/Game/BP_Hover` (`self.GetOwner`)))
  (set `self.Parent` _asbp_hover))

(event `self.ReceiveTick`
  (params (DeltaSeconds :type "Float (single-precision)"))
  (bind _returnvalue (`self.K2_GetComponentLocation`))
  (`/Engine/EditorBlueprintResources/StandardMacros.IsValid` (`self.Parent`)
    (:`Is Valid`
      (bind (_outhit _returnvalue_2) (`KismetSystemLibrary.LineTraceSingle` _returnvalue (- _returnvalue (* (`self.GetUpVector`) (`self.HoverDist`))) "TraceTypeQuery1"))
      (if _returnvalue_2
        (bind _output_get (set `self.HoverDelta` (- (`self.HoverDist`) (`.Distance` (`GameplayStatics.BreakHitResult` _outhit)))))
        (bind _asprimitive_component (cast `PrimitiveComponent` (`Actor.RootComponent` (`self.Parent`))))
        (`PrimitiveComponent.AddForceAtLocation` _asprimitive_component (* (`self.GetUpVector`) (+ (* (/ (- _output_get (`self.PrevHoverDelta`)) (`GameplayStatics.GetWorldDeltaSeconds`)) (`self.DampingCoefficent`)) (* _output_get (`self.SpringCoefficent`)))) (`self.K2_GetComponentLocation`) "None")
        (set `self.PrevHoverDelta` (`self.HoverDelta`))))))