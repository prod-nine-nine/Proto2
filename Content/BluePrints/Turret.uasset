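; Turret Blueprint with a custom Shoot event that fires a hitscan line trace for Pawn objects.
; The ray starts at the Gun component and runs toward the Scene component, with the normalized direction between them scaled by Range.
; The trace draws persistent debug lines and its hit result is unused, so no damage or effects follow.
; BeginPlay, overlap, Tick and the construction script are empty, and nothing here calls Shoot.
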(event `Shoot`
  (bind _returnvalue (`SceneComponent.K2_GetComponentLocation` (`self.Gun`)))
  (`KismetSystemLibrary.LineTraceSingleForObjects` :`Start` (`SceneComponent.K2_GetComponentLocation` (`self.Gun`)) :`End` (+ (* (`KismetMathLibrary.Normal` (- (`SceneComponent.K2_GetComponentLocation` (`self.Scene`)) _returnvalue)) (`self.Range`)) _returnvalue) :`ObjectTypes` (`|MakeArray` "ObjectTypeQuery3" :!type "EObjectTypeQuery Enum") :`DrawDebugType` "Persistent"))

(fn `UserConstructionScript`)