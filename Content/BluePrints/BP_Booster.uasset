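; BP_Booster is a thruster component that pushes its owner's root primitive along the component's up vector, at its own location.
; Each Use call applies Scale times Force times clamped delta time, trimming it once the frame's absolute total reaches the MaxForce budget.
; Tick resets both accumulators, saving the signed requested total, divided by a constant, as LastTotalForce and optionally printing it.
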(event `self.ReceiveBeginPlay`
  (set `self.Parent` (`self.GetOwner`)))

(event `self.ReceiveTick`
  (params (DeltaSeconds :type "Float (single-precision)"))
  (bind _totalforce (`self.TotalForce`))
  (set `self.TotalAbsForce` 0.0)
  (if (`self.Debug`)
    (`KismetSystemLibrary.PrintString` (`KismetStringLibrary.Conv_DoubleToString` _totalforce)))
  (set `self.lastTotalForce` (/ _totalforce 0.2))
  (set `self.TotalForce` 0.0))

(event `Use`
  (params (Scale :type "Float (double-precision)"))
  (bind _returnvalue (* Scale (`self.Force`) (`self.DeltaTime`)))
  (bind _returnvalue_2 (+ _returnvalue (`self.TotalForce`)))
  (bind _returnvalue_3 (+ (`KismetMathLibrary.Abs` _returnvalue) (`self.TotalAbsForce`)))
  (set `self.DeltaTime` (`KismetMathLibrary.FClamp` (`GameplayStatics.GetWorldDeltaSeconds`) 0.0 (`self.Delta time limit`)))
  (`/Engine/EditorBlueprintResources/StandardMacros.IsValid` (`self.Parent`)
    (:`Is Valid`
      (if (< _returnvalue 0.0)
        (set `self.Neg` -1.0)
        (else
          (set `self.Neg` 1.0)))
      (if (< (/ _returnvalue_3 (`self.DeltaTime`)) (`self.MaxForce`))
        (set `self.TotalForce` _returnvalue_2)
        (set `self.TotalAbsForce` _returnvalue_3)
        (bind _asprimitive_component (cast `PrimitiveComponent` (`Actor.RootComponent` (`self.Parent`))))
        (`PrimitiveComponent.AddForceAtLocation` _asprimitive_component (* (`self.GetUpVector`) _returnvalue) (`self.K2_GetComponentLocation`) "None")
        (else
          (set `self.TotalForce` _returnvalue_2)
          (bind _asprimitive_component_2 (cast `PrimitiveComponent` (`Actor.RootComponent` (`self.Parent`))))
          (`PrimitiveComponent.AddForceAtLocation` _asprimitive_component_2 (* (`self.GetUpVector`) (* (- (* (`self.MaxForce`) (`self.DeltaTime`)) (`self.TotalAbsForce`)) (`self.Neg`))) (`self.K2_GetComponentLocation`) "None")
          (set `self.TotalAbsForce` (* (`self.MaxForce`) (`self.DeltaTime`))))))))