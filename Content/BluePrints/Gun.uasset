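; Gun Blueprint that handles hitscan firing with limited ammo and a timed cooldown between shots.
; Shoot plays the fire animation, spends ammo, activates four muzzle flashes and line-traces from the skeleton toward a Scene component out to Range, ignoring the player pawn.
; Impact particles differ for BP_HoverAI hits versus everything else, and the struck actor is stored in HitActor without applying damage here.
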(event `self.ReceiveBeginPlay`)

(event `Shoot`
  (bind _gunskeleton (`self.GunSkeleton`))
  (bind _returnvalue (`SceneComponent.K2_GetComponentLocation` (`self.GunSkeleton`)))
  (if (and (> (`self.Ammo`) 0.0) (`self.canShoot`))
    (if (not (`SkeletalMeshComponent.IsPlaying` _gunskeleton))
      (`SkeletalMeshComponent.PlayAnimation` _gunskeleton "/Game/Animations/Attachments/QuadGun/An_QuadGun_Fire_Anim.An_QuadGun_Fire_Anim" false))
    (`/Engine/EditorBlueprintResources/StandardMacros.DecrementFloat` (`self.Ammo`)
      (:`  `
        (set `self.canShoot` false)
        (bind _outhit (`KismetSystemLibrary.LineTraceSingle` (+ (`SceneComponent.K2_GetComponentLocation` (`self.GunSkeleton`)) (0.0 0.0 20.0)) (+ (* (`KismetMathLibrary.Normal` (- (`SceneComponent.K2_GetComponentLocation` (`self.Scene`)) _returnvalue)) (`self.Range`)) (+ _returnvalue (0.0 0.0 20.0))) "TraceTypeQuery1" false (`|MakeArray` (`GameplayStatics.GetPlayerPawn` 0) :!type "Actor Object Reference") "ForDuration" true (struct :`R` 1.0 :`A` 1.0) (struct :`G` 1.0 :`A` 1.0) 0.1))
        (`ActorComponent.Activate` (`self.Pa_MuzzleFlash`) true)
        (`ActorComponent.Activate` (`self.Pa_MuzzleFlash1`) true)
        (`ActorComponent.Activate` (`self.Pa_MuzzleFlash2`) true)
        (`ActorComponent.Activate` (`self.Pa_MuzzleFlash3`) true)
        (cast `/Game/AI/BP_HoverAI` (`.HitActor` (`GameplayStatics.BreakHitResult` _outhit))
          (:`then`
            (`GameplayStatics.SpawnEmitterAtLocation` "/Game/VFX/Pa_BulletHit.Pa_BulletHit" (`.Location` (`GameplayStatics.BreakHitResult` _outhit))))
          (:`CastFailed`
            (`GameplayStatics.SpawnEmitterAtLocation` "/Game/VFX/Pa_BulletHitDust.Pa_BulletHitDust" (`.Location` (`GameplayStatics.BreakHitResult` _outhit)))))
        (set `self.HitActor` (`.HitActor` (`GameplayStatics.BreakHitResult` _outhit)))
        (`KismetSystemLibrary.Delay` (`self.SecondsBetweenShots`))
        (set `self.canShoot` true)))))

(fn `UserConstructionScript`)