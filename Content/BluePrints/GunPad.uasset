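; GunPad is a pickup pad that offers a random power-up to hover vehicles (BP_Hover).
; On BeginPlay it spawns a random Gun, LaserCannon, Shield or BigBoost and attaches it to the PickupDisplay, which spins every tick.
; When a hover vehicle without an attachment overlaps the capsule, the power-up moves to its AttachPoint socket and Attach is called.
; A timer then spawns a replacement three seconds later.
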(event `self.ReceiveBeginPlay`
  (`self.Spawn Gun`))

(event `self.ReceiveTick`
  (params (DeltaSeconds :type "Float (single-precision)"))
  (`SceneComponent.K2_AddRelativeRotation` (`self.PickupDisplay`) (struct :`Yaw` 1.0) false false))

(event `self.Capsule.OnComponentBeginOverlap`
  (params (OverlappedComponent :type "PrimitiveComponent Object Reference") (OtherActor :type "Actor Object Reference") (OtherComp :type "PrimitiveComponent Object Reference") (OtherBodyIndex :type Integer) (bFromSweep :type Boolean) (SweepResult :type "HitResult Structure (by ref)"))
  (`/Engine/EditorBlueprintResources/StandardMacros.IsValid` (`self.Current Power Up`)
    (:`Is Valid`
      (bind _asbp_hover (cast `/Game/BluePrints/BP_Hover` OtherActor))
      (`/Engine/EditorBlueprintResources/StandardMacros.IsValid` (`/Game/BluePrints/BP_Hover.Attachment` _asbp_hover)
        (:`Is Not Valid`
          (bind _output_get (set `/Game/BluePrints/BP_Hover.Attachment` (`self.Current Power Up`) _asbp_hover))
          (`self.K2_DetachFromActor` _output_get "KeepRelative" "KeepRelative" "KeepRelative")
          (`self.K2_AttachToComponent` _output_get (`/Game/BluePrints/BP_Hover.Vehicle` _asbp_hover) "AttachPoint" "KeepRelative" "KeepRelative" "KeepWorld" true)
          (bind _asattachment (cast `/Game/BluePrints/Attachment` _output_get))
          (`/Game/BluePrints/Attachment.Attach` _asattachment)
          (set `self.Current Power Up` null)
          (`KismetSystemLibrary.K2_SetTimerDelegate` (delegate `Spawn Gun`) 3.0))))))

(event `Spawn Gun`
  (bind _returnvalue (`SceneComponent.K2_GetComponentToWorld` (`self.PickupDisplay`)))
  (switch `int` (`KismetMathLibrary.RandomIntegerInRange` 0 3)
    (:`0`
      (bind _returnvalue_2 (`|SpawnActorFromClass` "/Game/BluePrints/Gun.Gun_C" _returnvalue "Undefined" "OverrideRootScale" null null))
      (set `self.Current Power Up` _returnvalue_2))
    (:`1`
      (bind _returnvalue_3 (`|SpawnActorFromClass` "/Game/BluePrints/LaserCannon.LaserCannon_C" _returnvalue "Undefined" "OverrideRootScale" null null))
      (set `self.Current Power Up` _returnvalue_3))
    (:`2`
      (bind _returnvalue_4 (`|SpawnActorFromClass` "/Game/BluePrints/Shield.Shield_C" _returnvalue "Undefined" "OverrideRootScale" null null))
      (set `self.Current Power Up` _returnvalue_4))
    (:`3`
      (bind _returnvalue_5 (`|SpawnActorFromClass` "/Game/BluePrints/BigBoost.BigBoost_C" _returnvalue "Undefined" "OverrideRootScale" null null))
      (set `self.Current Power Up` _returnvalue_5)))
  (`self.K2_AttachToComponent` (`self.Current Power Up`) (`self.PickupDisplay`) "None" "SnapToTarget" "SnapToTarget" "SnapToTarget" true))

(fn `UserConstructionScript`)