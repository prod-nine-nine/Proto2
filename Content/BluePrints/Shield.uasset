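; Shield Blueprint for an effect that grants a shield amount and shows it with a particle system.
; Activate works only while the Active flag is unset: it starts the particles, sets the flag and returns ShieldAmount, otherwise it returns zero.
; The Detach event hides the particle system and then calls the parent's Detach; nothing in these graphs clears the flag.
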(event `self.Detach`
  (`SceneComponent.SetVisibility` (`self.ParticleSystem`) false false)
  (`parent.Detach`))

(fn `Activate`
  (returns (ShieldAmount :type "Float (double-precision)"))
  (if (`self.Active`)
    (return 0.0)
    (else
      (`ActorComponent.Activate` (`self.ParticleSystem`) false)
      (set `self.Active` true)
      (return (`self.ShieldAmount`)))))

(fn `UserConstructionScript`
  (`parent.UserConstructionScript`))