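; Finish line actor that runs a hover race: start countdown, live player position and finish detection.
; BeginPlay gathers AI hovers plus the player, added last, and releases them after a delay.
; Tick ranks the player by straight-line distance to the line, adjusted for AI finishes, and declares a win if one racer remains.
; Player overlap ends the race with final placing, though its first-place win check is disabled.
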(event `self.ReceiveBeginPlay`
  (bind _racers (`self.Racers`))
  (bind _outactors (`GameplayStatics.GetAllActorsOfClass` "/Game/AI/BP_HoverAI.BP_HoverAI_C"))
  (set `self.Racers` _outactors)
  (bind _outactors_2 (`GameplayStatics.GetAllActorsOfClass` "/Game/BluePrints/BP_Hover.BP_Hover_C"))
  (bind _output (`|GetArrayItem` _outactors_2))
  (set `/Game/BluePrints/BP_Hover.InputEnabled` false _output)
  (`KismetArrayLibrary.Array_Add` _racers _output)
  (`KismetArrayLibrary.Array_Resize` (`self.RacerDistanceToFinish`) (`KismetArrayLibrary.Array_Length` _racers))
  (`KismetSystemLibrary.Delay` 4.5)
  (for _array_element (`self.Racers`)
    (bind _asbp_hover_ai (cast `/Game/AI/BP_HoverAI` _array_element)
      (:`then`
        (set `/Game/AI/BP_HoverAI.RaceStarted` true _asbp_hover_ai))
      (:`CastFailed`
        (bind _asbp_hover (cast `/Game/BluePrints/BP_Hover` _array_element))
        (set `/Game/BluePrints/BP_Hover.InputEnabled` true _asbp_hover)))))

(event `self.ReceiveActorBeginOverlap`
  (params (OtherActor :type "Actor Object Reference"))
  (if (not (`self.RaceFinished`))
    (cast `/Game/BluePrints/BP_Hover` OtherActor
      (:`then`
        (set `self.PlayerPos` (+ (`self.AIFinishes`) 1))
        (set `self.RaceFinished` true)
        (if (and (== (`self.PlayerPos`) 1) false)
          (set `self.PlayerWon` true)))
      (:`CastFailed`
        (bind _asbp_hover_ai (cast `/Game/AI/BP_HoverAI` OtherActor))
        (if (not (`/Game/AI/BP_HoverAI.RaceFinished` _asbp_hover_ai))
          (`/Engine/EditorBlueprintResources/StandardMacros.IncrementInt` (`self.AIFinishes`)))))))

(event `self.ReceiveTick`
  (params (DeltaSeconds :type "Float (single-precision)"))
  (bind _aifinishes (`self.AIFinishes`))
  (bind _racerdistancetofinish (`self.RacerDistanceToFinish`))
  (if (not (`self.RaceFinished`))
    (set `self.RacersAlive` 0)
    (for (_array_element _array_index) (`self.Racers`)
      (`/Engine/EditorBlueprintResources/StandardMacros.IsValid` _array_element
        (:`Is Valid`
          (`KismetArrayLibrary.Array_Set` (`self.RacerDistanceToFinish`) _array_index (`KismetMathLibrary.Vector_Distance` (`self.K2_GetActorLocation` _array_element) (`self.K2_GetActorLocation`)))
          (`/Engine/EditorBlueprintResources/StandardMacros.IncrementInt` (`self.RacersAlive`)))))
    (set `self.PlayerPos` 1)
    (for _array_element_2 (`self.RacerDistanceToFinish`)
      (if (< _array_element_2 (`|GetArrayItem` _racerdistancetofinish (`KismetArrayLibrary.Array_LastIndex` _racerdistancetofinish)))
        (`/Engine/EditorBlueprintResources/StandardMacros.IncrementInt` (`self.PlayerPos`))))
    (if (< (`self.PlayerPos`) _aifinishes)
      (set `self.PlayerPos` (+ _aifinishes 1)))
    ;[1 1 1] Player won by being last alive
    (if (== (`self.RacersAlive`) 1)
      (set `self.RaceFinished` true)
      (set `self.PlayerWon` true))))

(fn `UserConstructionScript`)