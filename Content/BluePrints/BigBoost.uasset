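; BigBoost is a booster Blueprint with an animated skeletal mesh and a fuel count that modifies a boost value passed into it.
; The first Activate call plays the booster supplement activation animation, sets Active and returns double the boost without checking fuel.
; Later calls return the boost unchanged, or zero once fuel runs out.
; UseFuel spends one fuel unit per call and reports whether any was available.
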(fn `Activate`
  (params (CurrentBoost :type "Float (double-precision)"))
  (returns (BoostAmount :type "Float (double-precision)"))
  (if (`self.Active`)
    (if (<= (`self.Fuel`) 0.0)
      (return 0.0)
      (else
        (return CurrentBoost)))
    (else
      (`SkeletalMeshComponent.PlayAnimation` (`self.SkeletalMesh`) "/Game/Animations/Attachments/BoosterSupplement/An_BoosterSupplement_Activate_Anim.An_BoosterSupplement_Activate_Anim" false)
      (set `self.Active` true)
      (return (* CurrentBoost 2.0)))))

(fn `useFuel`
  (returns (`Can Boost` :type Boolean))
  (if (> (`self.Fuel`) 0.0)
    (`/Engine/EditorBlueprintResources/StandardMacros.DecrementFloat` (`self.Fuel`)
      (:`  `
        (return true)))
    (else
      (return false))))

(fn `UserConstructionScript`
  (`parent.UserConstructionScript`))