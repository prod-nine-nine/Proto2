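; BP_HoverComponent is a scene component that hovers its owning actor above surfaces using spring-damper suspension.
; While On, each Tick traces down its local up axis and, on a hit, applies spring and damping force to the owner's root primitive at the component's location.
; A randomly timed looping event alternates hover distance between minimum and maximum while owner speed is at most 4000, varying the hover height.
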(event `self.ReceiveBeginPlay`
  (set `self.Parent` (`self.GetOwner`))
  (`KismetSystemLibrary.K2_SetTimerDelegate` (delegate `SwitchSwitch`) 0.3))

(event `SwitchSwitch`
  (if (<= (`KismetMathLibrary.VSize` (`Actor.GetVelocity` (`self.Parent`))) 4000.0)
    (bind _output_get (set `self.Switch` (not (`self.Switch`))))
    (if _output_get
      (set `self.HoverDist` (`self.MinHoverDist`))
      (else
        (set `self.HoverDist` (`self.MaxHoverDist`)))))
  (`KismetSystemLibrary.K2_SetTimerDelegate` (delegate `SwitchSwitch`) (`KismetMathLibrary.RandomFloatInRange` 0.1 0.5)))

(event `self.ReceiveTick`
  (params (DeltaSeconds :type "Float (single-precision)"))
  (bind _returnvalue (`self.K2_GetComponentLocation`))
  (bind _on (`self.On`))
  (if _on
    (`/Engine/EditorBlueprintResources/StandardMacros.IsValid` (`self.Parent`)
      (:`Is Valid`
        (bind (_outhit _returnvalue_2) (`KismetSystemLibrary.LineTraceSingle` _returnvalue (- _returnvalue (* (`self.GetUpVector`) (`self.HoverDist`))) "TraceTypeQuery1"))
        (bind _output_get (set `self.Grounded` _returnvalue_2))
        (if _output_get
          (bind _output_get_2 (set `self.HoverDelta` (- (`self.HoverDist`) (`.Distance` (`GameplayStatics.BreakHitResult` _outhit)))))
          (bind _asprimitive_component (cast `PrimitiveComponent` (`Actor.RootComponent` (`self.Parent`))))
          (`PrimitiveComponent.AddForceAtLocation` _asprimitive_component (* (`self.GetUpVector`) (+ (* (/ (- _output_get_2 (`self.PrevHoverDelta`)) (`KismetMathLibrary.FClamp` (`GameplayStatics.GetWorldDeltaSeconds`))) (`self.DampingCoefficent`)) (* _output_get_2 (`self.SpringCoefficent`)))) (`self.K2_GetComponentLocation`) "None")
          (set `self.PrevHoverDelta` (`self.HoverDelta`)))))
    (else
      (set `self.Grounded` _on))))