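; Laser cannon actor that fires a line trace once charged, limited by ammo and a cooldown between shots.
; Each Charge call builds ChargeAmount while ammo remains and shooting is allowed, firing at MaxCharge; Tick times the cooldown.
; Shoot traces Visibility from AttachmentMesh through the Scene component out to Range, ignoring the player pawn, and spends ammo.
; The trace draws a brief debug line, and its hit result is unused.
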(event `Charge`
  (if (and (> (`self.Ammo`) 0.0) (`self.canShoot`))
    (bind _result (`/Engine/EditorBlueprintResources/StandardMacros.IncrementFloat` (`self.ChargeAmount`))
      (:`  `
        (if (>= _result (`self.MaxCharge`))
          (set `self.ChargeAmount` 0.0)
          (set `self.Timer` 0.0)
          (`self.Shoot`))))))

(event `self.ReceiveTick`
  (params (DeltaSeconds :type "Float (single-precision)"))
  (if (not (`self.canShoot`))
    (set `self.Timer` (+ DeltaSeconds (`self.Timer`)))
    (if (>= (`self.Timer`) (`self.SecondsBetweenShots`))
      (set `self.canShoot` true))))

(event `Shoot`
  (bind _returnvalue (`SceneComponent.K2_GetComponentLocation` (`self.AttachmentMesh`)))
  (set `self.canShoot` false)
  (`KismetSystemLibrary.LineTraceSingle` (`SceneComponent.K2_GetComponentLocation` (`self.AttachmentMesh`)) (+ (* (`KismetMathLibrary.Normal` (- (`SceneComponent.K2_GetComponentLocation` (`self.Scene`)) _returnvalue)) (`self.Range`)) _returnvalue) "TraceTypeQuery1" false (`|MakeArray` (`GameplayStatics.GetPlayerPawn` 0) :!type "Actor Object Reference") "ForDuration" true (struct :`R` 1.0 :`A` 1.0) (struct :`G` 1.0 :`A` 1.0) 0.5)
  (`/Engine/EditorBlueprintResources/StandardMacros.DecrementFloat` (`self.Ammo`)))

(fn `UserConstructionScript`)