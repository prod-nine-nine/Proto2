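; Attachment actor that plays a drone attach animation and can later break off as a physics prop.
; Attach plays the animation on AttachSkel and reveals it after a brief delay; Tick hides it once playback ends and sets CanFunction.
; Detach makes AttachmentMesh blocking, detaches the actor, enables physics with a local force, then destroys it after DespawnTime.
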(event `self.ReceiveTick`
  (params (DeltaSeconds :type "Float (single-precision)"))
  (if (`self.IsAttached`)
    (if (not (or (`SkeletalMeshComponent.IsPlaying` (`self.AttachSkel`)) (`self.CanFunction`)))
      (`SceneComponent.SetVisibility` (`self.AttachSkel`) false false)
      (set `self.CanFunction` true))))

(event `Detach`
  (bind _attachmentmesh (`self.AttachmentMesh`))
  (`PrimitiveComponent.SetCollisionResponseToAllChannels` _attachmentmesh "ECR_Block")
  (`self.K2_DetachFromActor` "KeepWorld" "KeepWorld" "KeepWorld")
  (`PrimitiveComponent.SetSimulatePhysics` _attachmentmesh true)
  (`PrimitiveComponent.AddForceAtLocationLocal` _attachmentmesh (`self.Force`) (0.0 0.0 0.0) "None")
  (`KismetSystemLibrary.Delay` (`self.DespawnTime`))
  (`self.K2_DestroyActor`))

(event `Attach`
  (bind _attachskel (`self.AttachSkel`))
  (`SkeletalMeshComponent.PlayAnimation` _attachskel "/Game/Animations/Drone/An_Drone_Attach_Anim.An_Drone_Attach_Anim" false)
  (`KismetSystemLibrary.Delay` 0.2)
  (`SceneComponent.SetVisibility` _attachskel true false)
  (set `self.IsAttached` true))

(fn `UserConstructionScript`)