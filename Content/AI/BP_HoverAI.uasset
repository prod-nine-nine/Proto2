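; AI-driven hover vehicle that follows a sequence of track points, advancing its target on each TrackPointBetter overlap.
; While all six hover components are grounded, Tick interpolates yaw toward the current point and sets throttle.
; At high speed it projects velocity ahead and reverses thrust if that position lands farther from the following point.
; Booster components apply thrust, and velocity-based damping on zero input; airborne or past the last point, inputs are zero.
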(event `self.ReceiveBeginPlay`
  (bind _outactors (`GameplayStatics.GetAllActorsOfClass` "/Game/BluePrints/BP_Hover.BP_Hover_C"))
  (bind _output (`|GetArrayItem` _outactors))
  (`/Engine/EditorBlueprintResources/StandardMacros.IsValid` _output
    (:`Is Valid`
      (set `self.Player` _output))
    (:`Is Not Valid`
      _))
  (bind _outactors_2 (`GameplayStatics.GetAllActorsOfClass` "/Game/AI/TrackPoints.TrackPoints_C"))
  (bind _output_2 (`|GetArrayItem` _outactors_2))
  (`/Engine/EditorBlueprintResources/StandardMacros.IsValid` _output_2
    (:`Is Valid`
      (bind _output_get (set `self.TrackPoints` _output_2))
      (bind _trackpoints (`/Game/AI/TrackPoints.TrackPoints` _output_get))
      (set `self.TrackPointArray` _trackpoints)
      (set `self.NumTrackPoints` (`KismetArrayLibrary.Array_Length` _trackpoints)))))

(event `SetBoost`
  (params (BoostOn :type Boolean))
  (if BoostOn
    (set `self.BoostMultiplier` 1.8)
    (else
      (set `self.BoostMultiplier` 1.0))))

(event `InputAction|Reset`
  (params (Key :type "Key Structure")))

(event `InputAction|Boost`
  (params (Key :type "Key Structure")))

(event `InputAction|Aim`
  (params (Key :type "Key Structure"))
  (:`Pressed`
    (set `self.Aiming` true))
  (:`Released`
    (set `self.Aiming` false)))

(event `Accelerate`
  (params (`Axis Value` :type "Float (double-precision)"))
  ;[1 1 1] Acceleration
  (if (and (== `Axis Value` 0.0) (`self.Grounded`))
    (bind _returnvalue (`PrimitiveComponent.GetPhysicsLinearVelocity` (`self.Cube`) "None"))
    (bind _returnvalue_x (`KismetMathLibrary.BreakVector` (`KismetMathLibrary.InverseTransformDirection` (`self.GetTransform`) _returnvalue)))
    (`/Game/BluePrints/BP_Booster.Use` (`self.BoosterBLT`) (* _returnvalue_x -1.0 (`self.DampingMultiplier`)))
    (`/Game/BluePrints/BP_Booster.Use` (`self.BoosterBRT`) (* _returnvalue_x -1.0 (`self.DampingMultiplier`)))
    (`/Game/BluePrints/BP_Booster.Use` (`self.BoosterBLB`) (* _returnvalue_x -1.0 (`self.DampingMultiplier`)))
    (`/Game/BluePrints/BP_Booster.Use` (`self.BoosterBRB`) (* _returnvalue_x -1.0 (`self.DampingMultiplier`)))
    (else
      (`/Game/BluePrints/BP_Booster.Use` (`self.BoosterBLT`) (* `Axis Value` (`self.BoostMultiplier`)))
      (`/Game/BluePrints/BP_Booster.Use` (`self.BoosterBRT`) (* `Axis Value` (`self.BoostMultiplier`)))
      (`/Game/BluePrints/BP_Booster.Use` (`self.BoosterBLB`) (* `Axis Value` (`self.BoostMultiplier`)))
      (`/Game/BluePrints/BP_Booster.Use` (`self.BoosterBRB`) (* `Axis Value` (`self.BoostMultiplier`))))))

(event `self.ReceiveTick`
  (params (DeltaSeconds :type "Float (single-precision)"))
  (bind _returnvalue (`self.GetVelocity`))
  (bind (_returnvalue_roll _returnvalue_pitch) (`KismetMathLibrary.BreakRotator` (`self.K2_GetActorRotation`)))
  (bind _returnvalue_2 (+ (`self.CurrentPoint`) 1))
  (bind _returnvalue_3 (`self.K2_GetActorLocation` (`|GetArrayItem` (`self.TrackPointArray`) _returnvalue_2)))
  (bind (_returnvalue_roll_2 _returnvalue_pitch_2 _returnvalue_yaw) (`KismetMathLibrary.BreakRotator` (`KismetMathLibrary.RInterpTo` (`self.K2_GetActorRotation`) (`KismetMathLibrary.FindLookAtRotation` (`self.K2_GetActorLocation`) (`self.K2_GetActorLocation` (`|GetArrayItem` (`self.TrackPointArray`) (`self.CurrentPoint`)))) (`GameplayStatics.GetWorldDeltaSeconds`) 5.0)))
  (if (< (`self.CurrentPoint`) (`self.NumTrackPoints`))
    (set `self.Grounded` (and (`/Game/BluePrints/BP_HoverComponent.Grounded` (`self.HoverFL`)) (`/Game/BluePrints/BP_HoverComponent.Grounded` (`self.HoverFR`)) (`/Game/BluePrints/BP_HoverComponent.Grounded` (`self.HoverBL`)) (`/Game/BluePrints/BP_HoverComponent.Grounded` (`self.HoverBR`)) (`/Game/BluePrints/BP_HoverComponent.Grounded` (`self.HoverML`)) (`/Game/BluePrints/BP_HoverComponent.Grounded` (`self.HoverMR`))))
    (if (`self.Grounded`)
      (if (> (`KismetMathLibrary.VSize` _returnvalue) 2000.0)
        (set `self.PredictedPos` (+ (* _returnvalue 2.5) (`self.K2_GetActorLocation`)))
        (if (< _returnvalue_2 (`self.NumTrackPoints`))
          (set `self.CurrDistFromN+1` (`KismetMathLibrary.Vector_Distance` _returnvalue_3 (`self.K2_GetActorLocation`)))
          (set `self.PredictedDistFromN+1` (`KismetMathLibrary.Vector_Distance` (`self.PredictedPos`) _returnvalue_3))
          (if (> (`self.PredictedDistFromN+1`) (`self.CurrDistFromN+1`))
            (set `self.Acceleration` -1.0)
            (else
              (set `self.Acceleration` 0.5)))
          (else
            (set `self.Acceleration` 1.0 :!label _label)))
        (else
          (goto _label)))
      (`self.K2_SetActorRelativeRotation` (`KismetMathLibrary.MakeRotator` _returnvalue_roll _returnvalue_pitch _returnvalue_yaw))
      (`self.TurnRight` 0.0)
      (`self.Accelerate` (`self.Acceleration`))
      (`self.StrafeRight` 0.0)
      (else
        ;[1 1 1] Decelerate when not touching ground
        (`self.TurnRight` 0.0 :!label _label_2)
        (`self.Accelerate` 0.0)
        (`self.StrafeRight` 0.0)))
    (else
      (goto _label_2))))

(event `InputAxis|Foreward`
  (params (AxisValue :type "Float (single-precision)"))
  ;[1 1 1] Acceleration
)

(event `InputAction|ManuelHover`
  (params (Key :type "Key Structure"))
  (:`Pressed`
    (bind _output_get (set `self.Hovering` (not (`self.Hovering`))))
    (bind _output_get_2 (set `/Game/BluePrints/BP_HoverComponent.On` _output_get (`self.HoverBL`)))
    (bind _output_get_3 (set `/Game/BluePrints/BP_HoverComponent.On` _output_get_2 (`self.HoverFL`)))
    (bind _output_get_4 (set `/Game/BluePrints/BP_HoverComponent.On` _output_get_3 (`self.HoverFR`)))
    (bind _output_get_5 (set `/Game/BluePrints/BP_HoverComponent.On` _output_get_4 (`self.HoverBR`)))
    (bind _output_get_6 (set `/Game/BluePrints/BP_HoverComponent.On` _output_get_5 (`self.HoverML`)))
    (set `/Game/BluePrints/BP_HoverComponent.On` _output_get_6 (`self.HoverMR`))))

(event `TurnRight`
  (params (`Axis Value` :type "Float (double-precision)"))
  (bind (_returnvalue_x _returnvalue_y _returnvalue_z) (`KismetMathLibrary.BreakVector` (`PrimitiveComponent.GetPhysicsAngularVelocityInDegrees` (`self.Cube`) "None")))
  (bind _returnvalue (* `Axis Value` (`self.BoostMultiplier`)))
  (bind _returnvalue_2 (* `Axis Value` (`self.BoostMultiplier`)))
  (bind _returnvalue_3 (* _returnvalue_z -1.0 (`self.RotationDamping`)))
  ;[1 1 1] Turning
  (if (and (== `Axis Value` 0.0) (`self.Grounded`))
    (`/Game/BluePrints/BP_Booster.Use` (`self.BoosterFR`) _returnvalue_3)
    (`/Game/BluePrints/BP_Booster.Use` (`self.BoosterFL`) (* _returnvalue_3 -1.0))
    (elif (== (`self.GetInputAxisValue`) 0.0)
      (`/Game/BluePrints/BP_Booster.Use` (`self.BoosterFR`) _returnvalue_2)
      (`/Game/BluePrints/BP_Booster.Use` (`self.BoosterBRT`) _returnvalue_2)
      (`/Game/BluePrints/BP_Booster.Use` (`self.BoosterFL`) (* _returnvalue_2 -1.0))
      (`/Game/BluePrints/BP_Booster.Use` (`self.BoosterBLT`) (* _returnvalue_2 -1.0))
      (else
        (`/Game/BluePrints/BP_Booster.Use` (`self.BoosterBRT`) _returnvalue)
        (`/Game/BluePrints/BP_Booster.Use` (`self.BoosterBLT`) (* _returnvalue -1.0))))))

(event `self.ReceiveActorBeginOverlap`
  (params (OtherActor :type "Actor Object Reference"))
  (cast `/Game/AI/TrackPointBetter` OtherActor)
  (`/Engine/EditorBlueprintResources/StandardMacros.IncrementInt` (`self.CurrentPoint`)))

(event `StrafeRight`
  (params (`Axis Value` :type "Float (double-precision)"))
  ;[1 1 1] Strafing
  (if (and (== `Axis Value` 0.0) (`self.Grounded`))
    (bind _returnvalue (`PrimitiveComponent.GetPhysicsLinearVelocity` (`self.Cube`) "None"))
    (bind (_returnvalue_x _returnvalue_y) (`KismetMathLibrary.BreakVector` (`KismetMathLibrary.InverseTransformDirection` (`self.GetTransform`) _returnvalue)))
    (`/Game/BluePrints/BP_Booster.Use` (`self.BoosterSL`) (* _returnvalue_y -1.0 (`self.StrafeDamping`)))
    (`/Game/BluePrints/BP_Booster.Use` (`self.BoosterSR`) (* _returnvalue_y -1.0 (`self.StrafeDamping`)))
    (elif (`self.Grounded`)
      (`/Game/BluePrints/BP_Booster.Use` (`self.BoosterSL`) (* `Axis Value` (`self.BoostMultiplier`)))
      (`/Game/BluePrints/BP_Booster.Use` (`self.BoosterSR`) (* `Axis Value` (`self.BoostMultiplier`)))
      (else
        (`/Game/BluePrints/BP_Booster.Use` (`self.BoosterRL`) (* `Axis Value` (`self.BoostMultiplier`)))
        (`/Game/BluePrints/BP_Booster.Use` (`self.BoosterRR`) (* `Axis Value` (`self.BoostMultiplier`)))))))

(fn `UserConstructionScript`)