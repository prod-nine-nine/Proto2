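; Hover enemy AI pawn that moves toward AI_Hover pawns it sees.
; PawnSensing sightings that cast to AI_Hover start an AIMoveTo on that target, printing debug text on success or failure.
; BeginPlay caches the first TrackPoints actor found, but nothing here uses it afterward.
; A move toward the player character is present but never runs.
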(event `self.ReceiveBeginPlay`
  (bind _outactors (`GameplayStatics.GetAllActorsOfClass` "/Game/AI/TrackPoints.TrackPoints_C"))
  (bind _output (`|GetArrayItem` _outactors))
  (`/Engine/EditorBlueprintResources/StandardMacros.IsValid` _output
    (:`Is Valid`
      (set `self.TrackPoints` _output))))

(event `self.ReceiveTick`
  (params (DeltaSeconds :type "Float (single-precision)")))

(event `self.PawnSensing.OnSeePawn`
  (params (Pawn :type "Pawn Object Reference"))
  (bind _asai_hover (cast `/Game/AI/AI_Hover` Pawn))
  (`|AIMoveTo` self (0.0 0.0 0.0) _asai_hover
    (:`OnSuccess`
      (`KismetSystemLibrary.PrintString` "YAY"))
    (:`OnFail`
      (`KismetSystemLibrary.PrintString` "OHNO"))))

(fn `UserConstructionScript`)