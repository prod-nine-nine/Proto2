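; Booster component for BP_Hover that pushes the hover's root primitive along the booster's up vector at its own location.
; Use applies a signed, delta-time-scaled force each time it is called and accumulates the magnitude in TotalForce, which Tick resets.
; When a call would reach the MaxForce budget for that frame, it applies only the remaining force, preserving the sign.
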(event `self.ReceiveBeginPlay`
  (bind _asbp_hover (cast `/Game/BP_Hover` (`self.GetOwner`)))
  (set `self.Parent` _asbp_hover))

(event `self.ReceiveTick`
  (params (DeltaSeconds :type "Float (single-precision)"))
  (set `self.TotalForce` 0.0))

(event `Use`
  (params (Scale :type "Float (double-precision)"))
  (bind _returnvalue (* Scale (`self.Force`) (`GameplayStatics.GetWorldDeltaSeconds`)))
  (bind _returnvalue_2 (+ (`KismetMathLibrary.Abs` _returnvalue) (`self.TotalForce`)))
  (if (< _returnvalue 0.0)
    (set `self.Neg` -1.0)
    (else
      (set `self.Neg` 1.0)))
  (if (< (/ _returnvalue_2 (`GameplayStatics.GetWorldDeltaSeconds`)) (`self.MaxForce`))
    (set `self.TotalForce` _returnvalue_2)
    (bind _asprimitive_component (cast `PrimitiveComponent` (`Actor.RootComponent` (`self.Parent`))))
    (`PrimitiveComponent.AddForceAtLocation` _asprimitive_component (* (`self.GetUpVector`) _returnvalue) (`self.K2_GetComponentLocation`) "None")
    (else
      (bind _asprimitive_component_2 (cast `PrimitiveComponent` (`Actor.RootComponent` (`self.Parent`))))
      (`PrimitiveComponent.AddForceAtLocation` _asprimitive_component_2 (* (`self.GetUpVector`) (* (- (* (`self.MaxForce`) (`GameplayStatics.GetWorldDeltaSeconds`)) (`self.TotalForce`)) (`self.Neg`))) (`self.K2_GetComponentLocation`) "None")
      (set `self.TotalForce` (* (`self.MaxForce`) (`GameplayStatics.GetWorldDeltaSeconds`))))))